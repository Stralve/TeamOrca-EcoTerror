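; AI controller for an enemy that reacts to sound, running the BT_Hearing behavior tree from BeginPlay.
; Its AIPerception update handler acts only on successfully sensed hearing stimuli.
; Each one writes the stimulus location to the TargetLocation blackboard key for the tree, then calls AttackMessage followed by a Delay with nothing after it.
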(event OnTargetPerceptionUpdated(AIPerception)
  (params (Actor :type Actor%20Object%20Reference) (Stimulus :type AI%20Stimulus%20Structure))
  (bind (_age _expirationage _strength _stimuluslocation _receiverlocation _tag _bsuccessfullysensed) (Utilities|Struct|BreakAIStimulus Stimulus))
  (bind _returnvalue (Class|AIPerceptionSystem|GetSenseClassforStimulus Stimulus))
  (if (== _returnvalue "/Script/AIModule.AISense_Hearing")
    (if _bsuccessfullysensed
      (AI|Components|Blackboard|SetValueasVector (Variables|Default|GetBlackboard) (Utilities|Name|MakeLiteralName "TargetLocation") _stimuluslocation)
      (bind _anim_duration (Class|BIAttack|Attack(Message) self))
      (Utilities|FlowControl|Delay _anim_duration))))

(event EventBeginPlay
  (AI|RunBehaviorTree "/Game/TeamOrca/BrandonFolder/AI/BehaviorTree/BT_Hearing.BT_Hearing"))

(event EventTick
  (params (DeltaSeconds :type Float%20%28single-precision%29)))

(fn ConstructionScript)