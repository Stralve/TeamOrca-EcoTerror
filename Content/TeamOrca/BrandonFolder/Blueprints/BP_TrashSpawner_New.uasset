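; Trash spawner actor that scatters paper, can, bottle and bio items around itself on BeginPlay.
; For each type, it takes a fixed percentage of the total item count, then spawns at random offsets along its forward and right vectors, with ranges converted from feet to centimetres.
; Each item snaps to a short downward Visibility trace's hit location, without checking for a hit; the inclusive loop bound can add one extra per type.
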(event EventBeginPlay
  (Utilities|FlowControl|Sequence
    (:then_0
      (CallFunction|SetItemSpawnPercentage 50 "/Game/TeamOrca/Zeno/blueprints/BP_ItemPaper.BP_ItemPaper_C")
      (CallFunction|SpawnItems 7e+01 1e+02))
    (:then_1
      (CallFunction|SetItemSpawnPercentage 25 "/Game/TeamOrca/Zeno/blueprints/BP_ItemCans.BP_ItemCans_C")
      (CallFunction|SpawnItems 7e+01 1e+02))
    (:then_2
      (CallFunction|SetItemSpawnPercentage 20 "/Game/TeamOrca/Zeno/blueprints/BP_ItemBottles.BP_ItemBottles_C")
      (CallFunction|SpawnItems 7e+01 1e+02))
    (:then_3
      (CallFunction|SetItemSpawnPercentage 5 "/Game/TeamOrca/Zeno/blueprints/BP_ItemBio.BP_ItemBio_C")
      (CallFunction|SpawnItems 7e+01 1e+02))))

(fn ConstructionScript)

(fn SetItemSpawnPercentage
  (params (InPercentageToSpawn :type Integer) (Class%20To%20Spawn :type Actor%20Class%20Reference))
  (Variables|Default|SetItemToSpawn Class%20To%20Spawn)
  (Variables|Default|SetCurrentNumOfItemsToSpawn (* (/ InPercentageToSpawn 100) (Variables|Default|GetTotalNumItemsToSpawn)))
  (return))

(fn SpawnItems
  (params (InMaxDistanceToSpawnForwardInFeet :type Float%20%28double-precision%29) (InMaxDistanceToSpawnRightInFeet :type Float%20%28double-precision%29))
  (bind _distance_to_spawn_right (Variables|Default|GetDistance%20To%20Spawn%20Right))
  (bind _distance_to_spawn_forward (Variables|Default|GetDistance%20To%20Spawn%20Forward))
  (Utilities|SetMaxDistancetoSpawn InMaxDistanceToSpawnForwardInFeet InMaxDistanceToSpawnRightInFeet
    (:Return
      (for _index (range 0 (Variables|Default|GetCurrentNumOfItemsToSpawn))
        (bind _returnvalue (Game|SpawnActorfromClass (Variables|Default|GetItemToSpawn) (Math|Transform|MakeTransform (+ (Transformation|GetActorLocation) (+ (* (Transformation|GetActorForwardVector) (Math|Random|RandomFloatinRange (* _distance_to_spawn_forward -1.0) _distance_to_spawn_forward)) (* (Transformation|GetActorRightVector) (Math|Random|RandomFloatinRange (* _distance_to_spawn_right -1.0) _distance_to_spawn_right)))) "0, 0, 0" "1.000000,1.000000,1.000000") "AdjustIfPossibleButAlwaysSpawn" "MultiplyWithRoot" self 0))
        (bind _outhit (Collision|LineTraceByChannel (Transformation|GetActorLocation _returnvalue) (+ (Transformation|GetActorLocation _returnvalue) (* (Transformation|GetActorUpVector _returnvalue) "0.000000,0.000000,-100.000000")) "TraceTypeQuery1" false (Utilities|Array|MakeArray _returnvalue) "None"))
        (Transformation|SetActorLocation _returnvalue (.location _outhit) false false)))))