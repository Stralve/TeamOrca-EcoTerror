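; BP_Interactible is a generic interactable actor that the player can trigger while inside its sphere, whose radius is set on BeginPlay.
; Sphere overlaps track the most recent overlapping actor, and Interact proceeds only if that actor is the player character.
; It plays a sound and calls InteractFunction, a placeholder that only prints debug text.
; If DestroyOnInteract is set, it removes the sphere immediately and destroys the actor after a short delay.
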(event OnComponentBeginOverlap(Sphere)
  (params (OverlappedComponent :type Primitive%20Component%20Object%20Reference) (OtherActor :type Actor%20Object%20Reference) (OtherComp :type Primitive%20Component%20Object%20Reference) (OtherBodyIndex :type Integer) (bFromSweep :type Boolean) (SweepResult :type Hit%20Result%20Structure%20%28by%20ref%29))
  ;[1 1 1] Sets the overlapping actor
  (bind _output_get (Variables|Default|SetOverlappingActor OtherActor))
  ;[1 0 0] Debugging
  (Development|PrintString (Utilities|String|Append (Utilities|GetDisplayName _output_get) " can now interact with " (Utilities|GetDisplayName self))))

(event OnComponentEndOverlap(Sphere)
  (params (OverlappedComponent :type Primitive%20Component%20Object%20Reference) (OtherActor :type Actor%20Object%20Reference) (OtherComp :type Primitive%20Component%20Object%20Reference) (OtherBodyIndex :type Integer))
  ;[1 1 1] Checks if the overlapping actor is valid, if yes, sets it to empty
  (bind _overlappingactor (Variables|Default|GetOverlappingActor)
    (:then
      (if (== _overlappingactor OtherActor)
        (Variables|Default|SetOverlappingActor 0)))
    (:else)))

(event EventInteract
  ;[1 1 1] Checks if the overlapping actor is the player
  (bind _overlappingactor (Variables|Default|GetOverlappingActor)
    (:then
      (if (== _overlappingactor (Game|GetPlayerCharacter 0))
        ;[1 1 1] Plays Audio feedback
        (Audio|PlaySoundatLocation (Variables|Default|GetSound) (Transformation|GetActorLocation self) "0, 0, 0" 1.0 1.0 0.0 0 0 0 0)
        ;[1 1 1] Add Interact Function here
        (CallFunction|InteractFunction)
        ;[1 0 0] Needs Testing when interact key is working
        ;;[1 1 1] Checks if the interactible is destroyed when interacted or not
        (if (Variables|Default|GetDestroyOnInteract)
          ;;[1 1 1] Destroys the collision to prevent interaction during delay
          (Components|DestroyComponent (Variables|Default|GetSphere))
          (Utilities|FlowControl|Delay 0.1)
          (Actor|DestroyActor))))
    (:else)))

(event EventBeginPlay
  (Components|Sphere|SetSphereRadius (Variables|Default|GetSphere) (Variables|Components|GetIn%20Sphere%20Radius) true))

(fn ConstructionScript)

(fn InteractFunction
  ;[1 0 0] Debugging
  (Development|PrintString (Utilities|String|Append (Utilities|GetDisplayName self) " " "has been interacted"))
  (return))