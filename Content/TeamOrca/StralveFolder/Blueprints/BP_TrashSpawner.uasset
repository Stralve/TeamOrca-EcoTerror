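; BP_TrashSpawner is an actor that scatters a set number of BP_Item actors at random reachable navmesh points within a radius around itself.
; A fast looping timer started on BeginPlay spawns one item per tick, capped by a DoN on ItemsToSpawn.
; The timer-clearing branch sits behind the DoN exit, so the timer keeps looping after the cap.
; The construction script sizes a sphere component to match Radius.
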(event Custom|SpawnItem
  (bind _items_to_spawn (Variables|Default|GetItems%20to%20spawn))
  (bind _counter (Utilities|FlowControl|DoN _items_to_spawn)
    (:Exit
      (if (<= _counter _items_to_spawn)
        (Game|SpawnActorfromClass "/Game/TeamOrca/Zeno/blueprints/BP_Item.BP_Item_C" (Math|Transform|MakeTransform (.RandomLocation (AI|Navigation|GetRandomReachablePointinRadius (Transformation|GetActorLocation) (Variables|Default|GetRadius) 0 0)) "0, 0, 0" "1.000000,1.000000,1.000000") "Undefined" "MultiplyWithRoot" 0 0)
        (else
          (Utilities|Time|ClearandInvalidateTimerbyHandle (Variables|Default|GetNewVar)))))))

(event EventBeginPlay
  (bind _returnvalue (Utilities|Time|SetTimerbyEvent (delegate Custom|SpawnItem) 0.1 true))
  (Variables|Default|SetNewVar _returnvalue))

(fn ConstructionScript
  (Components|Sphere|SetSphereRadius (Variables|Default|GetSphere) (Variables|Default|GetRadius) true))