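; BP_CarLights is a toggleable car light built around a SpotLight component.
; On BeginPlay it applies the attenuation radius and outer cone angle from its variables to the spotlight.
; Each LightTrigger event runs a FlipFlop that alternates the intensity between zero and LightIntensity, switching the light off on the first call.
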(event EventLightTrigger
  (Utilities|FlowControl|FlipFlop
    (:A
      (Rendering|Components|Light|SetIntensity (Variables|Default|GetSpotLight) 0.0))
    (:B
      (Rendering|Components|Light|SetIntensity (Variables|Default|GetSpotLight) (Variables|Default|GetLightIntensity)))))

(event EventBeginPlay
  (bind _spotlight (Variables|Default|GetSpotLight))
  (Rendering|Lighting|SetAttenuationRadius _spotlight (Variables|Default|GetAttenuationRad))
  (Rendering|Lighting|SetOuterConeAngle _spotlight (Variables|Default|GetOuterConeAngle)))

(fn ConstructionScript)