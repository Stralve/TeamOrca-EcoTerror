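; BP_ItemPaper is a paper item actor that randomises its look and facing when play begins.
; BeginPlay calls the parent, sets a random entry from its Material array on the Cube mesh and gives the actor a random yaw across a full turn.
; Because RandomInteger receives the array's last index, whose value it excludes, the final material is never picked when there are several.
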(event EventBeginPlay
  (bind _material (Variables|Default|GetMaterial))
  (|CallParentFunction)
  (Rendering|Material|SetMaterial (Variables|Default|GetCube) 0 (Utilities|Array|Get(acopy) _material (Math|Random|RandomInteger (Utilities|Array|LastIndex _material))))
  (Transformation|SetActorRotation (Math|Rotator|MakeRotator 0.0 0.0 (Math|Random|RandomFloatinRange -1.8e+02 1.8e+02))))

(event Collision|EventActorBeginOverlap
  (params (OtherActor :type Actor%20Object%20Reference))
  (|CallParentFunction OtherActor) ; This node is disabled and will not be called.\nDrag off pins to build functionality.
)

(event EventTick
  (params (DeltaSeconds :type Float%20%28single-precision%29))
  (|CallParentFunction DeltaSeconds) ; This node is disabled and will not be called.\nDrag off pins to build functionality.
)

(fn ConstructionScript
  (|CallParentFunction))