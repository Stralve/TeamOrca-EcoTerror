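; BP_ItemBottles is a bottle item actor that varies its appearance by picking a random bottle mesh.
; Its construction script sets the Cube mesh component to a random entry from the Bottles array, so the mesh is re-rolled whenever construction reruns.
; The event graph adds no logic of its own, as BeginPlay only calls the parent and the overlap and tick events are disabled.
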(event EventBeginPlay
  (|CallParentFunction))

(event Collision|EventActorBeginOverlap
  (params (OtherActor :type Actor%20Object%20Reference))
  (|CallParentFunction OtherActor) ; This node is disabled and will not be called.\nDrag off pins to build functionality.
)

(event EventTick
  (params (DeltaSeconds :type Float%20%28single-precision%29))
  (|CallParentFunction DeltaSeconds) ; This node is disabled and will not be called.\nDrag off pins to build functionality.
)

(fn ConstructionScript
  (bind _bottles (Variables|Default|GetBottles))
  (|CallParentFunction)
  (Components|StaticMesh|SetStaticMesh (Variables|Default|GetCube) (Utilities|Array|Get(acopy) _bottles (Math|Random|RandomIntegerinRange 0 (Utilities|Array|LastIndex _bottles)))))