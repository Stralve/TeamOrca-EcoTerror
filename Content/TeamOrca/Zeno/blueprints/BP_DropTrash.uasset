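; BP_DropTrash is an interaction zone where the player drops one piece of carried trash per Interact press.
; Its box collision toggles input and a Gate as the player enters and leaves, so pressing Interact only works inside.
; A press finds the first BP_MainCharacter, decrements its TrashCount if above zero, then refreshes the fuel message on each assigned laser generator, printing a warning for invalid references.
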(event OnComponentBeginOverlap(Box_Collision)
  (params (OverlappedComponent :type Primitive%20Component%20Object%20Reference) (OtherActor :type Actor%20Object%20Reference) (OtherComp :type Primitive%20Component%20Object%20Reference) (OtherBodyIndex :type Integer) (bFromSweep :type Boolean) (SweepResult :type Hit%20Result%20Structure%20%28by%20ref%29))
  (bind _mainchar_ref (Variables|Default|GetMainChar%20Ref))
  (if (== OtherActor (Game|GetPlayerCharacter 0))
    (Input|EnableInput (Game|GetPlayerController 0))
    (Utilities|Casting|CastToBP_MainCharacter OtherActor)
    (Utilities|FlowControl|Gate true) ; enters at Open
  ))

(event OnComponentEndOverlap(Box_Collision)
  (params (OverlappedComponent :type Primitive%20Component%20Object%20Reference) (OtherActor :type Actor%20Object%20Reference) (OtherComp :type Primitive%20Component%20Object%20Reference) (OtherBodyIndex :type Integer))
  (bind _mainchar_ref (Variables|Default|GetMainChar%20Ref))
  (if (== OtherActor (Game|GetPlayerCharacter 0))
    (Input|DisableInput (Game|GetPlayerController 0))
    (Utilities|Casting|CastToBP_MainCharacter OtherActor)
    (Utilities|FlowControl|Gate true) ; enters at Close
  ))

(event Custom|Get%20Char%20Ref
  (bind _outactors (Actor|GetAllActorsOfClass "/Game/TeamOrca/BP_MainCharacter.BP_MainCharacter_C"))
  (Variables|Default|SetMainChar%20Ref (Utilities|Array|Get(acopy) _outactors)))

(event Collision|EventActorBeginOverlap
  (params (OtherActor :type Actor%20Object%20Reference)))

(event EventTick
  (params (DeltaSeconds :type Float%20%28single-precision%29)))

(event Input|ActionEvents|InputActionInteract
  (params (Key :type Key%20Structure :default "None"))
  (bind _mainchar_ref (Variables|Default|GetMainChar%20Ref))
  (:Pressed
    (Utilities|FlowControl|Gate true
      (:Exit
        (CallFunction|GetCharRef)
        (if (< 0 (Variables|/Game/TeamOrca/BP_MainCharacter.BP_MainCharacter_C|GetTrashCount _mainchar_ref))
          (bind _result (Math|Integer|DecrementInt (Variables|/Game/TeamOrca/BP_MainCharacter.BP_MainCharacter_C|GetTrashCount _mainchar_ref))
            (:%20%20
              (Variables|/Game/TeamOrca/BP_MainCharacter.BP_MainCharacter_C|SetTrashCount _mainchar_ref _result)
              (for _array_element (Variables|Default|GetLaserGenRef)
                (Utilities|IsValid _array_element
                  (:Is%20Valid
                    (Class|BPI-Lasers|UpdateFuel(Message) _array_element))
                  (:Is%20Not%20Valid
                    (Development|PrintString "Assign A Laser Generator")))))))))))

(fn ConstructionScript)