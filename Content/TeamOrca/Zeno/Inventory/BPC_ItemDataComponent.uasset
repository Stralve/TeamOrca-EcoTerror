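; Actor component for item actors that carries an item row handle and quantity for the inventory system.
; On BeginPlay it turns on replication for its owner.
; Interactwith is empty and LookAt returns an empty string.
; Pickup logic that adds the item to an inventory component and destroys the owner on success is present but disconnected, so it never runs.
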(event EventBeginPlay
  (Networking|SetReplicates (Components|GetOwner) true))

(event EventTick
  (params (DeltaSeconds :type Float%20%28single-precision%29)))

(event EventInteractwith
  (params (Player%20Character :type BP%20Main%20Character%20Object%20Reference)))

(fn Lookat
  (return ""))