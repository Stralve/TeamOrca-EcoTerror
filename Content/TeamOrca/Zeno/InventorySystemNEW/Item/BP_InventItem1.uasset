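; BP_InventItem1 is a world pickup actor for the inventory system that carries an Item value.
; On BeginPlay it passes the Item to its widget, apparently for a name prompt, which the Sphere shows and hides on any begin or end overlap.
; PickUpItem prints a debug message, triggers DestroyItem to remove the actor after a short delay, and returns the Item to the caller.
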(event OnComponentBeginOverlap(Sphere)
  (params (OverlappedComponent :type Primitive%20Component%20Object%20Reference) (OtherActor :type Actor%20Object%20Reference) (OtherComp :type Primitive%20Component%20Object%20Reference) (OtherBodyIndex :type Integer) (bFromSweep :type Boolean) (SweepResult :type Hit%20Result%20Structure%20%28by%20ref%29))
  (Rendering|SetVisibility (Variables|Default|GetWidget) true false))

(event OnComponentEndOverlap(Sphere)
  (params (OverlappedComponent :type Primitive%20Component%20Object%20Reference) (OtherActor :type Actor%20Object%20Reference) (OtherComp :type Primitive%20Component%20Object%20Reference) (OtherBodyIndex :type Integer))
  (Rendering|SetVisibility (Variables|Default|GetWidget) false false))

(event Custom|Destroy%20Item
  (Utilities|FlowControl|Delay 0.1)
  (Actor|DestroyActor))

(event EventBeginPlay
  (Class|BPIWidgetName|GetObjectNam(Message) (UserInterface|GetWidget (Variables|Default|GetWidget)) (Variables|Default|GetItem)))

(event Collision|EventActorBeginOverlap
  (params (OtherActor :type Actor%20Object%20Reference)))

(event EventTick
  (params (DeltaSeconds :type Float%20%28single-precision%29)))

(fn ConstructionScript)

(fn PickUpItem
  (Development|PrintString "Item Picked")
  (CallFunction|DestroyItem)
  (return (Variables|Default|GetItem)))